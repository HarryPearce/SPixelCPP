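; BP_Box_That_Takes_Damage is a damageable box actor in the Enemies folder that destroys itself when its health runs out.
; On AnyDamage, it destroys itself if Health is already at or below zero; otherwise it subtracts the damage and destroys itself once Health reaches zero or lower.
; The construction script is empty.
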(event `self.ReceiveAnyDamage`
  (params (Damage :type "Float (single-precision)") (DamageType :type "DamageType Object Reference") (InstigatedBy :type "Controller Object Reference") (DamageCauser :type "Actor Object Reference"))
  (if (<= (`self.Health`) 0.0)
    (`self.K2_DestroyActor`)
    (else
      (set `self.Health` (- (`self.Health`) Damage))
      (if (<= (`self.Health`) 0.0)
        (`self.K2_DestroyActor`)))))

(fn `UserConstructionScript`)