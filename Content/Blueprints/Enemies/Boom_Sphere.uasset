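; Boom_Sphere is a damageable explosive actor that blows up shortly after taking lethal damage.
; AnyDamage subtracts from Health until a hit would deplete it, then waits briefly, applies radial damage with falloff and destroys the actor.
; The blast is centered on the static mesh's relative location and uses the InnerRadius and OuterRadius variables.
; The construction script sizes two sphere components to match those radii.
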(event `self.ReceiveAnyDamage`
  (params (Damage :type "Float (single-precision)") (DamageType :type "DamageType Object Reference") (InstigatedBy :type "Controller Object Reference") (DamageCauser :type "Actor Object Reference"))
  (bind _returnvalue (- (`self.Health`) Damage))
  (if (<= _returnvalue 0.0)
    (`KismetSystemLibrary.Delay` 1.5)
    (`GameplayStatics.ApplyRadialDamageWithFalloff` :`BaseDamage` 40.0 :`MinimumDamage` 25.0 :`Origin` (`SceneComponent.RelativeLocation` (`self.StaticMeshComponent`)) :`DamageInnerRadius` (`self.Inner Radius`) :`DamageOuterRadius` (`self.OuterRadius`) :`DamageFalloff` 50.0 :`DamagePreventionChannel` "ECC_Camera")
    (`self.K2_DestroyActor`)
    (else
      (set `self.Health` _returnvalue))))

(fn `UserConstructionScript`
  (`SphereComponent.SetSphereRadius` (`self.Radius2`) (`self.Inner Radius`) true)
  (`SphereComponent.SetSphereRadius` (`self.Radius1`) (`self.OuterRadius`) true))