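; Damage cube that applies periodic damage to an overlapping actor.
; Begin overlap stores the latest actor and starts a Delay loop that damages it immediately, then every second while a flag is set.
; End overlap clears the flag after casting the player character, without checking which actor left.
; Health and shield check/damage macros are defined but unused in the event graph.
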(event `self.ReceiveActorBeginOverlap`
  (params (OtherActor :type "Actor Object Reference"))
  (bind _output_get (set `self.ActorReference` OtherActor))
  (set `self.PlayerInRadius` true)
  (if (`self.PlayerInRadius`) :!label _label
    (`GameplayStatics.ApplyDamage` _output_get 10.0)
    (`KismetSystemLibrary.Delay` 1.0)
    (goto _label)))

(event `self.ReceiveTick`
  (params (DeltaSeconds :type "Float (single-precision)")))

(event `self.ReceiveActorEndOverlap`
  (params (OtherActor :type "Actor Object Reference"))
  (cast `/Game/Blueprints/a_MainPlayer` (`GameplayStatics.GetPlayerCharacter` 0))
  (set `self.PlayerInRadius` false))

(fn `UserConstructionScript`)