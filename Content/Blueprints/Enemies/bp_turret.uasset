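; Enemy turret that turns toward the player on sight, fires three-shell bursts and is destroyed when health runs out.
; Sight and damage share one path: timelines lerp rotation toward the player, then back to the BeginPlay orientation after a retriggerable delay.
; Only sightings can fire: a SpawnProjectile toggle arms or starts a burst, telegraphed by a timed laser.
; Damage sets ReactingToDamage, so that path skips firing.
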(event `self.ReceiveAnyDamage`
  (params (Damage :type "Float (single-precision)") (DamageType :type "DamageType Object Reference") (InstigatedBy :type "Controller Object Reference") (DamageCauser :type "Actor Object Reference"))
  ;[1 1 1] See player, turn to them. No longer see, slowly reset.
  (set `self.Reacting_To_Damage` true)
  (bind _output_get (set `self.Current_Health` (- (`self.Current_Health`) Damage)))
  (if (<= _output_get 0.0)
    (`self.K2_DestroyActor`)
    (else
      (bind _asa_main_player (cast `/Game/Blueprints/a_MainPlayer` (stale `self.PawnSensing.OnSeePawn` Pawn) :!label _label))
      (`|ExecutionSequence`
        (:`then_0`
          (bind (_direction _newtrack_1) (`Timeline|Turret_Rotation_Reset` :!via `Stop` :!label _label_2)
            (:`Update`
              (bind _returnvalue (`KismetMathLibrary.FindLookAtRotation` (`self.K2_GetActorLocation`) (`self.K2_GetActorLocation` _asa_main_player)))
              (`self.K2_SetActorRotation` (`KismetMathLibrary.RLerp` _returnvalue (`KismetMathLibrary.MakeRotationFromAxes` (`self.Forward_Vector`) (`self.Right_Vector`) (`self.Up_Vector`)) _newtrack_1 true))
              (`ActorComponent.Deactivate` (`self.LaserSpawnPoint`)))))
        (:`then_1`
          (bind (_direction_2 _0_1_float) (`Timeline|Turret_Rotation_Rate` :!via `PlayFromStart`)
            (:`Update`
              (`self.K2_SetActorRotation` (`KismetMathLibrary.RLerp` (`KismetMathLibrary.Conv_VectorToRotator` (`SceneComponent.GetForwardVector` (`self.turret_top`))) _returnvalue _0_1_float true))
              (`KismetSystemLibrary.RetriggerableDelay` 2.0)
              (goto _label_2 :!via `PlayFromStart`))))
        (:`then_2`
          (if (`self.Reacting_To_Damage`)
            _
            (elif (`self.Spawn_Projectile`)
              (`KismetSystemLibrary.Delay` (- (`self.Fire_Rate`) (`self.Laser_On_Time`)))
              (`ActorComponent.Activate` (`self.Laser`) false)
              (`KismetSystemLibrary.Delay` (`self.Laser_On_Time`))
              (`ActorComponent.Deactivate` (`self.Laser`))
              (`|SpawnActorFromClass` "/Game/Blueprints/Enemies/bp_projectile_shell.bp_projectile_shell_C" (`SceneComponent.K2_GetComponentToWorld` (`self.ProjectileSpawnPoint`)) "AdjustIfPossibleButAlwaysSpawn" "OverrideRootScale")
              (`KismetSystemLibrary.Delay` 0.2)
              (`|SpawnActorFromClass` "/Game/Blueprints/Enemies/bp_projectile_shell.bp_projectile_shell_C" (`SceneComponent.K2_GetComponentToWorld` (`self.ProjectileSpawnPoint`)) "AdjustIfPossibleButAlwaysSpawn" "OverrideRootScale")
              (`KismetSystemLibrary.Delay` 0.2)
              (`|SpawnActorFromClass` "/Game/Blueprints/Enemies/bp_projectile_shell.bp_projectile_shell_C" (`SceneComponent.K2_GetComponentToWorld` (`self.ProjectileSpawnPoint`)) "AdjustIfPossibleButAlwaysSpawn" "OverrideRootScale")
              (set `self.Spawn_Projectile` false)
              (else
                (set `self.Spawn_Projectile` true)))))))))

(event `self.PawnSensing.OnSeePawn`
  (params (Pawn :type "Pawn Object Reference"))
  ;[1 1 1] See player, turn to them. No longer see, slowly reset.
  (set `self.Reacting_To_Damage` false)
  (goto _label))

(event `self.ReceiveBeginPlay`
  (bind _capsulecomponent (`self.CapsuleComponent`))
  ;[1 1 1] At start set vectors, health
  (set `self.Forward_Vector` (`SceneComponent.GetForwardVector` _capsulecomponent))
  (set `self.Up_Vector` (`SceneComponent.GetUpVector` _capsulecomponent))
  (set `self.Right_Vector` (`SceneComponent.GetRightVector` _capsulecomponent))
  (`/Engine/EditorBlueprintResources/StandardMacros.DoOnce` false
    (:`Completed`
      (set `self.Current_Health` (`self.Max_Health`)))))

(fn `UserConstructionScript`)