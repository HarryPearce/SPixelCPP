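; Healbox is an actor that gradually restores the main player's health on overlap.
; On begin overlap it casts to a_MainPlayer, then adds a small amount to CurrentPlayerHealth in a short Delay loop until it reaches MaxPlayerHealth.
; The loop has no end-overlap check or clamp, so healing continues after the player leaves and can slightly overshoot the maximum.
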(event `self.ReceiveActorBeginOverlap`
  (params (OtherActor :type "Actor Object Reference"))
  (bind _asa_main_player (cast `/Game/Blueprints/a_MainPlayer` OtherActor))
  (if (< (`/Game/Blueprints/a_MainPlayer.CurrentPlayerHealth` _asa_main_player) (`/Game/Blueprints/a_MainPlayer.MaxPlayerHealth` _asa_main_player)) :!label _label
    (set `/Game/Blueprints/a_MainPlayer.CurrentPlayerHealth` (+ (`/Game/Blueprints/a_MainPlayer.CurrentPlayerHealth` _asa_main_player) 0.5) _asa_main_player)
    (`KismetSystemLibrary.Delay` 0.01)
    (goto _label)))

(fn `UserConstructionScript`
  (`parent.UserConstructionScript`))