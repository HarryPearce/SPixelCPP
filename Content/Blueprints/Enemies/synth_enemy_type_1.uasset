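; Synth enemy character that chases a seen player via pawn sensing and repeats delayed sphere-trace melee attacks while the player is in range.
; Any, radial and point damage handlers route hits to shield or health, with brief invulnerability and ragdoll, capsule removal or destruction on death.
; Shield logic appears copied from the player: input toggles it, Tick regenerates it, and some helpers alter the player character's speed or shield.
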(event `InputAction|Attack1`
  (params (Key :type "Key Structure" :default "AnyKey"))
  ;[1 1 1] Debug Raytrace
)

(event `self.ReceiveBeginPlay`
  (set `self.Synth` self))

(event `self.PawnSensing.OnSeePawn`
  (params (Pawn :type "Pawn Object Reference"))
  (if (not (`self.Attacking_Player`))
    (bind _asa_main_player (cast `/Game/Blueprints/a_MainPlayer` Pawn))
    (`|AIMoveTo` self (0.0 0.0 0.0) _asa_main_player 10.0 true)))

(event `self.Attack_Range.OnComponentBeginOverlap`
  (params (OverlappedComponent :type "PrimitiveComponent Object Reference") (OtherActor :type "Actor Object Reference") (OtherComp :type "PrimitiveComponent Object Reference") (OtherBodyIndex :type Integer) (bFromSweep :type Boolean) (SweepResult :type "HitResult Structure (by ref)"))
  (bind _attack_range (`self.Attack_Range`))
  (bind _returnvalue (`SceneComponent.K2_GetComponentLocation` _attack_range))
  (cast `/Game/Blueprints/a_MainPlayer` OtherActor)
  (set `self.Player_In_Range` true)
  (set `self.Attacking_Player` true :!label _label)
  (`KismetSystemLibrary.Delay` (`self.Swing_Timer`))
  (bind _outhit (`KismetSystemLibrary.SphereTraceSingle` _returnvalue (+ _returnvalue (* (`SceneComponent.GetForwardVector` _attack_range) (`self.Attack_Distance_Multiplier`))) 50.0 "TraceTypeQuery1"))
  (`GameplayStatics.ApplyDamage` (`.HitActor` (`GameplayStatics.BreakHitResult` _outhit)) (`self.Base_Damage`))
  (set `self.Attacking_Player` false)
  (if (`self.Player_In_Range`)
    (goto _label)))

(event `self.Attack_Range.OnComponentEndOverlap`
  (params (OverlappedComponent :type "PrimitiveComponent Object Reference") (OtherActor :type "Actor Object Reference") (OtherComp :type "PrimitiveComponent Object Reference") (OtherBodyIndex :type Integer))
  (set `self.Player_In_Range` false))

(event `self.ReceiveAnyDamage`
  (params (Damage :type "Float (single-precision)") (DamageType :type "DamageType Object Reference") (InstigatedBy :type "Controller Object Reference") (DamageCauser :type "Actor Object Reference"))
  ;[1 1 1] Any damage taken, check shield - if shield damage shield, if not then health
  (if (`self.Invulnerable`)
    _
    (elif (`self.IsShieldPressed`)
      (`self.CheckShield`
        (:`true`
          (`self.CheckHealth` :!label _label
            (:`true`
              ;[1 1 1] Damage player, then kill if needed. Also set brief invuln to avoid over damage
              (`self.DamageHealth` Damage
                (:`True`
                  (set `self.Invulnerable` true)
                  (`KismetSystemLibrary.Delay` (`self.InvulnTimer`))
                  (set `self.Invulnerable` false))
                (:`false`
                  (`self.PlayerDeath`))))
            (:`false`
              (`ActorComponent.K2_DestroyComponent` (`Character.CapsuleComponent` (`self.Synth`))))))
        (:`false`
          ;[1 1 1] Set shield to damage, then timer on regen. Also check if broken then set broken / invuln if needed
          (set `self.ShieldDamageTaken` true)
          (`self.DamageShield` Damage
            (:`True`
              (`self.CheckShieldBroken`)
              (set `self.Invulnerable` true)
              (`KismetSystemLibrary.Delay` 0.5)
              (set `self.Invulnerable` false))
            (:`false`
              (`KismetSystemLibrary.RetriggerableDelay` (`self.ShieldRegenTrigger`))
              (set `self.ShieldDamageTaken` false)))))
      (else
        (goto _label)))))

(event `self.ReceiveRadialDamage`
  (params (DamageReceived :type "Float (single-precision)") (DamageType :type "DamageType Object Reference") (Origin :type "Vector Structure") (HitInfo :type "HitResult Structure (by ref)") (InstigatedBy :type "Controller Object Reference") (DamageCauser :type "Actor Object Reference"))
  ;[1 1 1] Any damage taken, check shield - if shield damage shield, if not then health
  (if (`self.Invulnerable`)
    _
    (elif (`self.IsShieldPressed`)
      (`self.CheckShield`
        (:`true`
          (`self.CheckHealth` :!label _label_2
            (:`true`
              ;[1 1 1] Damage player, then kill if needed. Also set brief invuln to avoid over damage
              (`self.DamageHealth` DamageReceived
                (:`True`
                  (set `self.Invulnerable` true)
                  (`KismetSystemLibrary.Delay` (`self.InvulnTimer`))
                  (set `self.Invulnerable` false))
                (:`false`
                  (`self.PlayerDeath`))))
            (:`false`
              (`PrimitiveComponent.SetSimulatePhysics` (`self.Mesh`) true)
              (`KismetSystemLibrary.Delay` 5.0)
              (`ActorComponent.K2_DestroyComponent` (`Character.CapsuleComponent` (`self.Synth`))))))
        (:`false`
          ;[1 1 1] Set shield to damage, then timer on regen. Also check if broken then set broken / invuln if needed
          (set `self.ShieldDamageTaken` true)
          (`self.DamageShield` DamageReceived
            (:`True`
              (`self.CheckShieldBroken`)
              (set `self.Invulnerable` true)
              (`KismetSystemLibrary.Delay` 0.5)
              (set `self.Invulnerable` false))
            (:`false`
              (`KismetSystemLibrary.RetriggerableDelay` (`self.ShieldRegenTrigger`))
              (set `self.ShieldDamageTaken` false)))))
      (else
        (goto _label_2)))))

(event `self.ReceivePointDamage`
  (params (Damage :type "Float (single-precision)") (DamageType :type "DamageType Object Reference") (HitLocation :type "Vector Structure") (HitNormal :type "Vector Structure") (HitComponent :type "PrimitiveComponent Object Reference") (BoneName :type Name) (ShotFromDirection :type "Vector Structure") (InstigatedBy :type "Controller Object Reference") (DamageCauser :type "Actor Object Reference") (HitInfo :type "HitResult Structure (by ref)"))
  ;[1 1 1] Any damage taken, check shield - if shield damage shield, if not then health
  (if (`self.Invulnerable`)
    _
    (elif (`self.IsShieldPressed`)
      (`self.CheckShield`
        (:`true`
          (`self.CheckHealth` :!label _label_3
            (:`true`
              ;[1 1 1] Damage player, then kill if needed. Also set brief invuln to avoid over damage
              (`self.DamageHealth` Damage
                (:`True`
                  (set `self.Invulnerable` true)
                  (`KismetSystemLibrary.Delay` (`self.InvulnTimer`))
                  (set `self.Invulnerable` false))
                (:`false`
                  (`self.PlayerDeath`))))
            (:`false`
              (`self.K2_DestroyActor`))))
        (:`false`
          ;[1 1 1] Set shield to damage, then timer on regen. Also check if broken then set broken / invuln if needed
          (set `self.ShieldDamageTaken` true)
          (`self.DamageShield` Damage
            (:`True`
              (`self.CheckShieldBroken`)
              (set `self.Invulnerable` true)
              (`KismetSystemLibrary.Delay` 0.5)
              (set `self.Invulnerable` false))
            (:`false`
              (`KismetSystemLibrary.RetriggerableDelay` (`self.ShieldRegenTrigger`))
              (set `self.ShieldDamageTaken` false)))))
      (else
        (goto _label_3)))))

(event `InputAction|Shield`
  (params (Key :type "Key Structure" :default "AnyKey"))
  (bind _player0shield (`self.Player0Shield`))
  (bind _shieldvisible (`self.ShieldVisible`))
  ;[1 1 1] Ensure the shield is not broken, then appropriately set the shield status
  (:`Pressed`
    (if (not (`self.ShieldBroken`))
      (set `self.IsShieldPressed` true)
      (if (not _shieldvisible)
        ;[1 1 1] Check if the shield is visible / can collide and adjust as the button is pushed or released
        (`SceneComponent.ToggleVisibility` _player0shield false)
        (set `self.ShieldVisible` true)
        (`self.ShieldSlowPlayer`)
        (`self.ShieldNoCollide`))))
  (:`Released`
    (set `self.IsShieldPressed` false)
    (if _shieldvisible
      (`SceneComponent.ToggleVisibility` _player0shield false)
      (set `self.ShieldVisible` false)
      (`self.ShieldSlowPlayer`)
      (`self.ShieldNoCollide`))))

(event `self.ReceiveTick`
  (params (DeltaSeconds :type "Float (single-precision)"))
  ;[1 1 1] Event Tick to regen shield at proper rate
  (`|ExecutionSequence`
    (:`then_0`
      (if (`self.ShieldBroken`)
        (`KismetSystemLibrary.Delay` (`self.ShieldRegenRate`))
        (`self.ShieldRegen_Broken`)
        (elif (not (`self.IsShieldPressed`))
          (`KismetSystemLibrary.Delay` (`self.ShieldRegenRate`))
          (`self.ShieldRegen`))))))

(fn `Calculatehealth`
  (params (`Delta Health` :type "Float (double-precision)") (`Delta Shield` :type "Float (double-precision)"))
  (returns (NewParam :type "Float (double-precision)"))
  (return 0.0))

(fn `CheckShieldBroken`
  (if (<= (`self.CurrentShield`) 0.0)
    (set `self.ShieldBroken` true)
    (set `self.IsShieldPressed` false)
    (if (`self.ShieldVisible`)
      (bind _asa_main_player (cast `/Game/Blueprints/a_MainPlayer` (`GameplayStatics.GetPlayerCharacter` 0)))
      (`SceneComponent.ToggleVisibility` (`/Game/Blueprints/a_MainPlayer.Player0Shield` _asa_main_player) false)
      (set `self.ShieldVisible` false)
      (`self.ShieldSlowPlayer`)
      (`self.ShieldNoCollide`))))

(fn `NewFunction_1`
  (returns (Output_Get :type "Float (double-precision)"))
  (if (`self.ShieldDamageTaken`)
    _
    (elif (not (>= (`self.CurrentShield`) (`self.MaxShield`)))
      (bind _output_get (set `self.CurrentShield` (+ (`self.CurrentShield`) (* (`self.MaxShield`) (`|GetArrayItem` (`self.ShieldRegenAMT`))))))
      (return _output_get))))

(fn `PlayerDeath`
  (`CharacterMovementComponent.DisableMovement` (`self.CharacterMovement`))
  (`PrimitiveComponent.SetSimulatePhysics` (`self.Mesh`) true))

(fn `RayTrace`
  (returns (Output_Get :type "Actor Object Reference"))
  (bind _returnvalue (`GameplayStatics.GetPlayerCameraManager` 0))
  (bind _returnvalue_2 (`SceneComponent.K2_GetComponentLocation` (`PlayerCameraManager.TransformComponent` _returnvalue)))
  ;[1 1 1] Store hit actor
  (bind (_outhit _returnvalue_3) (`KismetSystemLibrary.LineTraceSingle` :`Start` _returnvalue_2 :`End` (+ _returnvalue_2 (* (`SceneComponent.GetForwardVector` (`PlayerCameraManager.TransformComponent` _returnvalue)) (`self.MaxUseDistance`))) :`TraceChannel` "TraceTypeQuery1" :`DrawDebugType` "ForDuration"))
  (if _returnvalue_3
    (bind _output_get (set `self.ActorTraced` (`.HitActor` (`GameplayStatics.BreakHitResult` _outhit))))
    (return _output_get)
    (else
      (set `self.ActorTraced` null))))

(fn `ShieldNoCollide`
  (bind _player0shield (`self.Player0Shield`))
  (if (`self.ShieldVisible`)
    (`PrimitiveComponent.SetCollisionEnabled` _player0shield "QueryAndPhysics")
    (else
      (`PrimitiveComponent.SetCollisionEnabled` _player0shield "NoCollision"))))

(fn `ShieldRegen`
  (returns (Output_Get :type "Float (double-precision)"))
  (if (`self.ShieldDamageTaken`)
    _
    (elif (not (>= (`self.CurrentShield`) (`self.MaxShield`)))
      (bind _output_get (set `self.CurrentShield` (+ (`self.CurrentShield`) (* (`self.MaxShield`) (`|GetArrayItem` (`self.ShieldRegenAMT`))))))
      (return _output_get))))

(fn `ShieldRegen_Broken`
  (if (< (`self.CurrentShield`) (* (`self.MaxShield`) 0.2))
    (set `self.CurrentShield` (+ (`self.CurrentShield`) (* (`self.MaxShield`) (`|GetArrayItem` (`self.ShieldRegenAMT`) 1))))
    (else
      (set `self.ShieldBroken` false))))

(fn `ShieldSlowPlayer`
  (bind _charactermovement (`Character.CharacterMovement` (`GameplayStatics.GetPlayerCharacter` 0)))
  (if (`self.ShieldVisible`)
    (set `CharacterMovementComponent.MaxWalkSpeed` 100.0 _charactermovement)
    (else
      (set `CharacterMovementComponent.MaxWalkSpeed` 600.0 _charactermovement))))

(fn `UserConstructionScript`
  (`self.ShieldNoCollide`))