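; Actor Blueprint that turns a referenced static mesh into a procedural mesh with collision.
; The construction script assigns the mesh to a static mesh component, copies it into the procedural mesh component, then destroys the static mesh component.
; BeginPlay prints the section count and stores the first section's vertices, triangles and normals in variables, with no further use of them here.
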(event `self.ReceiveBeginPlay`
  (`KismetSystemLibrary.PrintString` (`KismetStringLibrary.Conv_IntToString` (`ProceduralMeshComponent.GetNumSections` (`self.ProceduralMesh`))))
  (bind (_vertices _triangles _normals) (`KismetProceduralMeshLibrary.GetSectionFromStaticMesh` (`self.StaticMeshRef`)))
  (set `self.NewVar_0` _vertices)
  (set `self.NewVar_1` _triangles)
  (set `self.NewVar_2` _normals)
  (`KismetSystemLibrary.PrintString` "Hello"))

(fn `UserConstructionScript`
  (`StaticMeshComponent.SetStaticMesh` (`self.StaticMesh`) (`self.StaticMeshRef`))
  (`KismetProceduralMeshLibrary.CopyProceduralMeshFromStaticMeshComponent` (`self.StaticMesh`) 0 (`self.ProceduralMesh`) true)
  (`ActorComponent.K2_DestroyComponent` (`self.StaticMesh`)))