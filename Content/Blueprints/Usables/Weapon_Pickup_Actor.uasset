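; Weapon pickup actor in the usables set that creates a weapon object from its configured weapon class.
; On BeginPlay it constructs the weapon with the game instance as outer and stores it, then manually forwards its own Tick to that object each frame.
; The use handler only passes through to the parent implementation, so this Blueprint adds no pickup logic of its own.
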(event `self.ReceiveBeginPlay`
  (`parent.ReceiveBeginPlay`)
  (bind _returnvalue (`|GenericCreateObject` (`self.WeaponClass_0`) (`GameplayStatics.GetGameInstance`) null "0.000000,0.000000,0.000000|0.000000,0.000000,0.000000|1.000000,1.000000,1.000000"))
  (set `self.Weapon_0` _returnvalue))

(event `self.ReceiveTick`
  (params (DeltaSeconds :type "Float (single-precision)"))
  (`/Game/Blueprints/Weapons/Abstract/Weapon.Tick` (`self.Weapon_0`) DeltaSeconds))

(fn `OnActorUsed`
  (params (Controller :type "PlayerController Object Reference"))
  (returns (Success :type Boolean))
  (bind _success (`parent.OnActorUsed` Controller))
  (return _success))

(fn `UserConstructionScript`
  (`parent.UserConstructionScript`))