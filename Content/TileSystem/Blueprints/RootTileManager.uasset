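; Root tile manager that procedurally builds levels by joining streamed tile-level instances at connection points.
; GenerateTile reads the tile DataTable, aligns connectors, rejects overlaps using a temporary box component, then creates the level instance.
; InstanceShown initialises the new tile's untagged TileManager and broadcasts completion.
; CreateTileGraph places a random starting tile and target marker; GenerateCriticalPathStep picks random connector tiles that move closer to the target.
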(event `self.ReceiveBeginPlay`
  (`self.Init` null)
  (set `self.RootTileManager` self)
  (`BlueprintMapLibrary.Map_Add` (`self.IdTileManagerMap`) "root" self)
  (set `self.RandomStream` (`KismetMathLibrary.MakeRandomStream` (`KismetMathLibrary.RandomInteger` 200000))))

(fn `AddTileManager`
  (params (TM :type "/Game/TileSystem/Blueprints/TileManager Object Reference"))
  (locals (TMA :type "/Game/TileSystem/Blueprints/TileManagerArray Object Reference") (_TM :type "/Game/TileSystem/Blueprints/TileManager Object Reference"))
  (bind __tm (`local._TM`))
  (bind _output_get (set `local._TM` TM))
  (bind (_value _returnvalue) (`BlueprintMapLibrary.Map_Find` (`self.TileDepthMap`) (`/Game/TileSystem/Blueprints/TileManager.Depth` _output_get)))
  (set `local.TMA` _value)
  (if (not _returnvalue)
    (bind _returnvalue_2 (`|GenericCreateObject` "/Game/TileSystem/Blueprints/TileManagerArray.TileManagerArray_C" self))
    (set `local.TMA` _returnvalue_2)
    (`BlueprintMapLibrary.Map_Add` (`self.TileDepthMap`) (`/Game/TileSystem/Blueprints/TileManager.Depth` (`local._TM`)) (`local.TMA`)))
  (`KismetArrayLibrary.Array_Add` (`/Game/TileSystem/Blueprints/TileManagerArray.Value` (`local.TMA`)))
  (`BlueprintMapLibrary.Map_Add` (`self.IdTileManagerMap`) (`/Game/TileSystem/Blueprints/TileManager.TileId` __tm) __tm))

(fn `CreateTileGraph`
  (params (StartPosition :type "Vector Structure") (TargetPosition :type "Vector Structure") (PathDefinitions :type "Array of /Game/TileSystem/PathDefinition Structure") (GraphName :type String))
  (locals (StartConnectorId :type String) (StartingTileNames :type "Array of Name") (StartingTileName :type Name))
  (for _array_element PathDefinitions
    (if (`|EnumEquality` (`.PathType_2_A7C1650349DA6D809D30AF9F62978D31` (break `/Game/TileSystem/PathDefinition` _array_element)) "NewEnumerator0")
      (`KismetArrayLibrary.Array_Add` (`self.CurrentlyGeneratedCriticalPaths`) _array_element)
      (else
        (`KismetArrayLibrary.Array_Add` (`self.CurrentlyGeneratedNonCriticalPaths`) _array_element))))
  (set `local.StartConnectorId` GraphName)
  (bind _output_get (set `self.CurrentGraphGenerationTargetLocation` TargetPosition))
  (`|SpawnActorFromClass` "/Game/TileSystem/Blueprints/TileGenerationTargetMarker.TileGenerationTargetMarker_C" (`KismetMathLibrary.MakeTransform` _output_get) "Undefined" "OverrideRootScale" null null)
  (bind _returnvalue (`|SpawnActorFromClass` "/Game/TileSystem/Blueprints/ConnectionPoint.ConnectionPoint_C" (`KismetMathLibrary.MakeTransform` StartPosition (`KismetMathLibrary.MakeRotator` 0.0 0.0 (`KismetMathLibrary.RandomFloatInRange` -179.0 179.0))) "Undefined" "OverrideRootScale" null (`local.StartConnectorId`) false null))
  (bind _output_get_2 (set `self.CurrentGraphGenerationStartPoint` _returnvalue))
  (set `/Game/TileSystem/Blueprints/TileElement.ParentTileManager` self _output_get_2)
  (`BlueprintMapLibrary.Map_Add` (`self.ConnectionPoints`) (`local.StartConnectorId`) _output_get_2)
  (bind (_tilename _connectorinfo) (`self.GetTileGenerationParameters` (`BlueprintGameplayTagLibrary.MakeGameplayTagQuery` (struct :`TagDictionary` (struct :`(TagName` "StartingTile")) :`QueryTokenStream` "(0,1,1,1,0)" :`AutoDescription` " ANY( StartingTile )"))))
  (add `self.TileGenerated` (`|CreateDelegate` :!event `GenerateCriticalPathStep`))
  (bind _success (`self.GenerateTile` "" self _tilename (`.Name_12_ED608672476F3ED7C2C7F0A0E54C214A` (break `/Game/TileSystem/ConnectorInfo` _connectorinfo)) (`local.StartConnectorId`)))
  (if _success
    _))

(fn `GenerateCriticalPathStep`
  (locals (CurrentlyGeneratedPath :type "/Game/TileSystem/PathDefinition Structure") (ClosestPointToTarget :type "/Game/TileSystem/Blueprints/ConnectionPoint Object Reference") (ClosestPointToTargetDistance :type "Float (double-precision)" :default 0.0) (TargetConnector :type "/Game/TileSystem/ConnectorInfo Structure") (TargetConnectorSet :type Boolean) (NewTileName :type Name) (ValidTiles :type "Array of Name"))
  (clear `self.TileGenerated`)
  (if (< (`self.CurrentlyGeneratedCriticalPathIndex`) (`KismetArrayLibrary.Array_Length` (`self.CurrentlyGeneratedCriticalPaths`)))
    (set `local.CurrentlyGeneratedPath` (`|GetArrayItem` (`self.CurrentlyGeneratedCriticalPaths`) (`self.CurrentlyGeneratedCriticalPathIndex`)))
    (if (<= (`KismetArrayLibrary.Array_Length` (`self.GetOverlappingActors` (`self.LastTileManager`) "/Game/TileSystem/Blueprints/TileGenerationTargetMarker.TileGenerationTargetMarker_C")) 0)
      (bind _free_connectors (`self.GetFreeConnectors` (`self.LastTileManager`)))
      (bind (_closestpoint1 _closestdistance1) (`self.GetConnectorClosestToLocation` _free_connectors (`self.CurrentGraphGenerationTargetLocation`)))
      (set `local.ClosestPointToTarget` _closestpoint1)
      (set `local.ClosestPointToTargetDistance` _closestdistance1)
      (bind _tilenames (`self.GetTilesWithTag` (struct :`TagDictionary` (struct :`(TagName` "ConnectorTile")) :`QueryTokenStream` "(0,1,1,1,0)" :`AutoDescription` " ANY( ConnectorTile )")))
      (set `local.ValidTiles` _tilenames)
      (while (and (> (`KismetArrayLibrary.Array_Length` (`local.ValidTiles`)) 0) (not (`local.TargetConnectorSet`)))
        (bind _output (`self.GetRandomName` (`local.ValidTiles`)))
        (bind _output_get (set `local.NewTileName` _output))
        (bind _returnvalue (`|GetDataTableRow` "/Game/TileSystem/TileInfoTable.TileInfoTable" _output_get)
          (:`then`
            (bind _values (`BlueprintMapLibrary.Map_Values` (`.Connectors_7_F55D331D46CB58E05CD363B1019C6AE9` (break `/Game/TileSystem/TileInfo` _returnvalue))))
            (for _array_element _values
              (bind (_tilerotation _levellocation _connectorlocation) (`self.CalculateTileTransform` (`local.ClosestPointToTarget`) _array_element))
              (`KismetSystemLibrary.LineTraceSingle` :`Start` _connectorlocation :`End` (`KismetMathLibrary.MakeVector` (.x _connectorlocation) (.y _connectorlocation) 1000.0) :`TraceChannel` "TraceTypeQuery1" :`DrawDebugType` "Persistent")
              (if (< (`KismetMathLibrary.VSize` (- _connectorlocation (`self.CurrentGraphGenerationTargetLocation`))) (`local.ClosestPointToTargetDistance`))
                (set `local.TargetConnector` _array_element)
                (set `local.TargetConnectorSet` true)))
            (if (not (`local.TargetConnectorSet`))
              (`KismetArrayLibrary.Array_RemoveItem` (`local.ValidTiles`) (`local.NewTileName`))
              (set `local.NewTileName` "None")))))
      (add `self.TileGenerated` (`|CreateDelegate` :!event `GenerateCriticalPathStep`))
      (`self.GenerateTile` "" (`self.LastTileManager`) (`KismetStringLibrary.Conv_NameToString` (`local.NewTileName`)) (`.Name_12_ED608672476F3ED7C2C7F0A0E54C214A` (break `/Game/TileSystem/ConnectorInfo` (`local.TargetConnector`))) (`/Game/TileSystem/Blueprints/ConnectionPoint.Name` (`local.ClosestPointToTarget`)))
      (else
        (`KismetSystemLibrary.PrintString` "Done")
        (bind _outactors (`GameplayStatics.GetAllActorsOfClass` "/Game/TileSystem/Blueprints/TileGenerationTargetMarker.TileGenerationTargetMarker_C"))
        (`self.K2_DestroyActor` _outactors)))))

(fn `GenerateTile`
  (params (TileId :type String) (TileManager :type "/Game/TileSystem/Blueprints/TileManager Object Reference") (TileNameToGenerate :type String) (TargetConnectorName :type String) (SourceConnectorName :type String))
  (returns (Success :type Boolean))
  (locals (_TM :type "/Game/TileSystem/Blueprints/TileManager Object Reference") (TN :type String) (SCN :type String) (InstanceName :type String) (LSI :type "LevelStreaming Object Reference") (TCN :type String) (TargetConnectorLocation :type "Vector Structure") (TargetConnectorInfo :type "/Game/TileSystem/ConnectorInfo Structure") (TileInfo :type "/Game/TileSystem/TileInfo Structure") (LevelLocation :type "Vector Structure") (LevelRotation :type "Rotator Structure") (BC :type "BoxComponent Object Reference"))
  (bind _scn (`local.SCN`))
  (bind _inoverlappingcomponents (`PrimitiveComponent.GetOverlappingComponents` (`local.BC`)))
  (bind _value (`BlueprintMapLibrary.Map_Find` (`self.IdTileManagerMap`) TileId))
  (bind (_tilerotation _levellocation) (`self.CalculateTileTransform` (`self.SourceConnector`) (`local.TargetConnectorInfo`)))
  (bind (_value_2 _returnvalue) (`BlueprintMapLibrary.Map_Find` (`/Game/TileSystem/Blueprints/TileManager.ConnectionPoints` (`local._TM`)) _scn))
  ;[1 1 1] Don't generate tile if one is in progress
  (if (not (`self.CurrentlyGeneratingTile`))
    (set `self.CurrentlyGeneratingTile` true)
    ;[1 1 1] Var Init
    (set `self.TileNameToCreate` TileNameToGenerate)
    (set `local.SCN` SourceConnectorName)
    (set `self.TargetConnectorName` TargetConnectorName)
    (set `local.TN` TileNameToGenerate)
    (bind _output_get (set `local._TM` TileManager))
    ;[1 1 1] Find Tile Manager to connect new tile to
    (`/Engine/EditorBlueprintResources/StandardMacros.IsValid` _output_get
      (:`Is Valid`
        _)
      (:`Is Not Valid`
        (`/Engine/EditorBlueprintResources/StandardMacros.IsValid` _value
          (:`Is Valid`
            (set `local._TM` _value))
          (:`Is Not Valid`
            (`KismetSystemLibrary.PrintString` "Error: Tile Manager Not Found - Cannot Generate Tile")
            (set `self.CurrentlyGeneratingTile` false)
            ;[1 1 1] Find tile to generate info
            (return false)))))
    (bind _returnvalue_2 (`|GetDataTableRow` "/Game/TileSystem/TileInfoTable.TileInfoTable" (`KismetStringLibrary.Conv_StringToName` (`self.TileNameToCreate`)))
      (:`then`
        (bind _output_get_2 (set `local.TileInfo` _returnvalue_2))
        (bind (_value_3 _returnvalue_3) (`BlueprintMapLibrary.Map_Find` (`.Connectors_7_F55D331D46CB58E05CD363B1019C6AE9` (break `/Game/TileSystem/TileInfo` _output_get_2)) (`self.TargetConnectorName`)))
        ;[1 1 1] Find Connector to connec to in new tile
        (if _returnvalue_3
          (bind _output_get_3 (set `local.TargetConnectorInfo` _value_3))
          (if (`.Disabled_17_9486DDFB4A1AA67337C4469FF52B935D` (break `/Game/TileSystem/ConnectorInfo` _output_get_3))
            (`KismetSystemLibrary.PrintString` "Error: Target connector not found in infotable - Cannot Generate Tile" :!label _label)
            (set `self.CurrentlyGeneratingTile` false)
            ;[1 1 1] Find Connector to connect from in the existing tile
            (return false)
            (elif _returnvalue
              (set `self.SourceConnector` _value_2)
              (bind _result (`/Engine/EditorBlueprintResources/StandardMacros.IncrementInt` (`self.GenerationIndex`))
                (:`  `
                  (set `self.TileIdToCreate` (`KismetStringLibrary.Concat_StrStr` (`self.TileNameToCreate`) "_" (`KismetStringLibrary.Conv_IntToString` _result)))
                  (set `local.LevelRotation` _tilerotation)
                  (set `local.LevelLocation` _levellocation)
                  (bind _returnvalue_4 (`AddComponent|NODE_AddBoxComponent-0`))
                  (bind _output_get_4 (set `local.BC` _returnvalue_4))
                  (`PrimitiveComponent.SetCollisionProfileName` _output_get_4 "BoundaryCheckPreset")
                  (`PrimitiveComponent.SetCollisionEnabled` _output_get_4 "QueryAndPhysics")
                  (for _array_element (`.BoundaryDefinitions_11_6B3F2C664FE67D31772C3686D0119D95` (break `/Game/TileSystem/TileInfo` (`local.TileInfo`)))
                    (bind (_boxextent _boxlocation _rotation) (break `/Game/TileSystem/BoundaryInfo` _array_element))
                    (`SceneComponent.K2_SetWorldLocation` (`local.BC`) (+ _boxlocation (`local.LevelLocation`)) false true)
                    (`SceneComponent.K2_SetWorldRotation` (`local.BC`) (`KismetMathLibrary.NormalizedDeltaRotator` (`local.LevelRotation`) _rotation) false false)
                    (`BoxComponent.SetBoxExtent` (`local.BC`) (- _boxextent (2.0 2.0 2.0)) true)
                    (if (> (`KismetArrayLibrary.Array_Length` _inoverlappingcomponents) 0)
                      (for _array_element_2 _inoverlappingcomponents
                        (bind _asbox_collision (cast `BoxComponent` _array_element_2))
                        (`SceneComponent.SetHiddenInGame` _asbox_collision false false))
                      (`SceneComponent.SetHiddenInGame` (`local.BC`) false false)
                      (`KismetSystemLibrary.PrintString` "Cannot GenerateTile - Overlap Detected")
                      (return false)))
                  (`ActorComponent.K2_DestroyComponent` (`local.BC`))
                  (bind _returnvalue_5 (`LevelStreaming.CreateInstance` (`GameplayStatics.GetStreamingLevel` (`KismetStringLibrary.Conv_StringToName` (`self.TileNameToCreate`))) (`self.TileIdToCreate`)))
                  (bind _output_get_5 (set `self.CurrentlyGeneratedInstance` _returnvalue_5))
                  (`KismetSystemLibrary.PrintString` (`KismetTextLibrary.Conv_TextToString` (`|FormatText` "SC Rot: {SCROT} SC Inverted: {SCINV} TC Rot {TCROT} Rot Delta {RDelta}" (`KismetTextLibrary.Conv_StringToText` (`KismetStringLibrary.Conv_RotatorToString` (struct))) (`KismetTextLibrary.Conv_StringToText` (`KismetStringLibrary.Conv_RotatorToString` (struct))) (`KismetTextLibrary.Conv_StringToText` (`KismetStringLibrary.Conv_RotatorToString` (struct))) (`KismetTextLibrary.Conv_StringToText` (`KismetStringLibrary.Conv_RotatorToString` _tilerotation)))) false true (struct :`G` 0.66 :`B` 1.0 :`A` 1.0) 30.0)
                  (`KismetSystemLibrary.PrintString` (`KismetTextLibrary.Conv_TextToString` (`|FormatText` "SC Loc {SCLOC} TC Loc {TCLOC} Rotated TC loc {RLOC} Combined Loc {CLOC}" (`KismetTextLibrary.Conv_StringToText` (`KismetStringLibrary.Conv_VectorToString` (0.0 0.0 0.0))) (`KismetTextLibrary.Conv_StringToText` (`KismetStringLibrary.Conv_VectorToString` (0.0 0.0 0.0))) (`KismetTextLibrary.Conv_StringToText` (`KismetStringLibrary.Conv_VectorToString` (0.0 0.0 0.0))) (`KismetTextLibrary.Conv_StringToText` (`KismetStringLibrary.Conv_VectorToString` _levellocation)))) false true (struct :`G` 0.66 :`B` 1.0 :`A` 1.0) 30.0)
                  (set `LevelStreaming.LevelTransform` (`KismetMathLibrary.MakeTransform` _levellocation _tilerotation) _output_get_5)
                  (add `LevelStreaming.OnLevelShown` (`self.CurrentlyGeneratedInstance`) (`|CreateDelegate` :!event `InstanceShown`))
                  (set `LevelStreaming.bShouldBeLoaded` true (`self.CurrentlyGeneratedInstance`))
                  (set `LevelStreaming.bShouldBeVisible` true (`self.CurrentlyGeneratedInstance`))
                  (`KismetSystemLibrary.PrintString` (`KismetTextLibrary.Conv_TextToString` (`|FormatText` "Source Connector: {SCN} Target ConnectorName: {TCN} TileNameToCreate {TNTC} TileIdToCreate {TIDTC}" (`KismetTextLibrary.Conv_StringToText` (`/Game/TileSystem/Blueprints/ConnectionPoint.Name` (`self.SourceConnector`))) (`KismetTextLibrary.Conv_StringToText` (`self.TargetConnectorName`)) (`KismetTextLibrary.Conv_StringToText` (`self.TileNameToCreate`)) (`KismetTextLibrary.Conv_StringToText` (`self.TileIdToCreate`)))) false true (struct :`G` 0.66 :`B` 1.0 :`A` 1.0) 30.0)))
              (else
                (`KismetSystemLibrary.PrintString` (`KismetStringLibrary.Concat_StrStr` "Error: Source connector not found - Cannot Generate Tile - " _scn))
                (set `self.CurrentlyGeneratingTile` false)
                (return false))))
          (else
            (goto _label))))
      (:`RowNotFound`
        (`KismetSystemLibrary.PrintString` "Error: Tile not found in infotable - Cannot Generate Tile")
        (set `self.CurrentlyGeneratingTile` false)
        (return false)))))

(fn `GetConnectorClosestToLocation`
  (params (Connector :type "Array of /Game/TileSystem/Blueprints/ConnectionPoint Object Reference") (Location :type "Vector Structure"))
  (returns (ClosestPoint1 :type "/Game/TileSystem/Blueprints/ConnectionPoint Object Reference") (ClosestDistance1 :type "Float (double-precision)"))
  (locals (ClosestDistance :type "Float (double-precision)" :default -1.0) (ClosestPoint :type "/Game/TileSystem/Blueprints/ConnectionPoint Object Reference"))
  (bind _closestdistance (`local.ClosestDistance`))
  (for _array_element Connector
    (bind _returnvalue (`KismetMathLibrary.VSize` (- (`self.K2_GetActorLocation` _array_element) Location)))
    (if (or (< _returnvalue _closestdistance) (== _closestdistance -1.0))
      (set `local.ClosestDistance` _returnvalue)
      (set `local.ClosestPoint` _array_element)))
  (return (`local.ClosestPoint`) (`local.ClosestDistance`)))

(fn `GetRandomConnector`
  (params (Array :type "Array of /Game/TileSystem/ConnectorInfo Structure"))
  (returns (Output :type "/Game/TileSystem/ConnectorInfo Structure"))
  (return (`|GetArrayItem` Array (`KismetMathLibrary.RandomIntegerFromStream` (`KismetArrayLibrary.Array_Length` Array) (`self.RandomStream`)))))

(fn `GetRandomName`
  (params (Array :type "Array of Name"))
  (returns (Output :type Name))
  (return (`|GetArrayItem` Array (`KismetMathLibrary.RandomIntegerFromStream` (`KismetArrayLibrary.Array_Length` Array) (`self.RandomStream`)))))

(fn `GetTilesWithTag`
  (params (Query :type "GameplayTagQuery Structure"))
  (returns (TileNames :type "Array of Name"))
  (locals (_TileNames :type "Array of Name"))
  (bind _outrownames (`DataTableFunctionLibrary.GetDataTableRowNames` "/Game/TileSystem/TileInfoTable.TileInfoTable"))
  (for _array_element _outrownames
    (bind _returnvalue (`|GetDataTableRow` "/Game/TileSystem/TileInfoTable.TileInfoTable" _array_element)
      (:`then`
        (if (`BlueprintGameplayTagLibrary.DoesContainerMatchTagQuery` (`.Flags_19_2C7B79C446CA8B148917C594364A0CD9` (break `/Game/TileSystem/TileInfo` _returnvalue)) Query)
          (`KismetArrayLibrary.Array_Add` (`local._TileNames`) _array_element)))))
  (return (`local._TileNames`)))

(fn `InstanceShown`
  (bind _outactors (`GameplayStatics.GetAllActorsOfClass` "/Game/TileSystem/Blueprints/TileManager.TileManager_C"))
  (for _array_element _outactors
    (if (not (`BlueprintGameplayTagLibrary.HasTag` (`/Game/TileSystem/Interfaces/TaggableActor.OwnedTags` _array_element) (struct :`TagName` "TileAssigned")))
      (bind _output_get (set `self.LastTileManager` _array_element))
      (`self.Init` _array_element (`self.SourceConnector`) (`self.TargetConnectorName`) (`self.TileNameToCreate`) (`self.TileIdToCreate`))
      (`self.Init` _output_get (`self.SourceConnector`) (`self.TargetConnectorName`) (`self.TileNameToCreate`) (`self.TileIdToCreate`))
      (set `self.CurrentlyGeneratingTile` false)
      (break)))
  (`self.TileGenerated`))

(fn `UserConstructionScript`
  (`parent.UserConstructionScript`))