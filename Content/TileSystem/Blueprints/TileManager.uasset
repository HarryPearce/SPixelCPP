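; TileManager represents one tile in a connected tile tree, tracking its name, ID, depth, elements and connection points.
; Init derives depth from the parent connector, registers with the root manager, then processes all TileElement actors in the world.
; Elements matching a tag query are claimed and tagged TileAssigned; connection points are mapped by name, with the named one linked back to the parent.
; GetFreeConnectors returns enabled, unlinked connection points.
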(fn `GetConnectionPoints`
  (returns (ConnectionPOints :type "Array of /Game/TileSystem/Blueprints/ConnectionPoint Object Reference"))
  (bind _values (`BlueprintMapLibrary.Map_Values` (`self.ConnectionPoints`)))
  (return _values))

(fn `GetFreeConnectors`
  (returns (`Free Connectors` :type "Array of /Game/TileSystem/Blueprints/ConnectionPoint Object Reference"))
  (locals (Ret :type "Array of /Game/TileSystem/Blueprints/ConnectionPoint Object Reference"))
  (bind _values (`BlueprintMapLibrary.Map_Values` (`self.ConnectionPoints`)))
  (for _array_element _values
    (`/Engine/EditorBlueprintResources/StandardMacros.IsValid` (`/Game/TileSystem/Blueprints/ConnectionPoint.ConnectedConnector` _array_element)
      (:`Is Not Valid`
        (if (not (`/Game/TileSystem/Blueprints/ConnectionPoint.Disabled` _array_element))
          (`KismetArrayLibrary.Array_Add` (`local.Ret`) _array_element)))))
  (return (`local.Ret`)))

(fn `Init`
  (params (ConnectedFrom :type "/Game/TileSystem/Blueprints/ConnectionPoint Object Reference") (ConnectedToName :type String) (TileName :type String) (TileId :type String))
  (locals (_ConnectedFrom :type "/Game/TileSystem/Blueprints/ConnectionPoint Object Reference") (_ConnectedToName :type String))
  (bind _parenttilemanager (`/Game/TileSystem/Blueprints/TileElement.ParentTileManager` (`local._ConnectedFrom`)))
  (set `self.TileName` TileName)
  (set `self.TileId` TileId)
  (bind _output_get (set `local._ConnectedFrom` ConnectedFrom))
  (set `local._ConnectedToName` ConnectedToName)
  (`/Engine/EditorBlueprintResources/StandardMacros.IsValid` _output_get
    (:`Is Valid`
      (bind _output_get_2 (set `self.ParentTileManager` _parenttilemanager))
      (set `self.Depth` (+ (`/Game/TileSystem/Blueprints/TileManager.Depth` _output_get_2) 1))
      (bind _output_get_3 (set `self.RootTileManager` (`/Game/TileSystem/Blueprints/TileManager.RootTileManager` _parenttilemanager)))
      (`/Game/TileSystem/Blueprints/RootTileManager.AddTileManager` _output_get_3 self))
    (:`Is Not Valid`
      _))
  (bind _outactors (`GameplayStatics.GetAllActorsOfClass` "/Game/TileSystem/Blueprints/TileElement.TileElement_C"))
  (for _array_element _outactors
    (if (`BlueprintGameplayTagLibrary.DoesContainerMatchTagQuery` (`/Game/TileSystem/Interfaces/TaggableActor.OwnedTags` _array_element) (`self.TagQuery`))
      (`KismetArrayLibrary.Array_Add` (`self.TileElements`) _array_element)
      (`BlueprintGameplayTagLibrary.AddGameplayTag` (`/Game/TileSystem/Interfaces/TaggableActor.OwnedTags` _array_element) (struct :`TagName` "TileAssigned"))
      (set `/Game/TileSystem/Blueprints/TileElement.ParentTileManager` self _array_element)
      (bind _asconnection_point (cast `/Game/TileSystem/Blueprints/ConnectionPoint` _array_element))
      (`BlueprintMapLibrary.Map_Add` (`self.ConnectionPoints`) (`/Game/TileSystem/Blueprints/ConnectionPoint.Name` _asconnection_point) _asconnection_point)
      (if (`KismetStringLibrary.EqualEqual_StrStr` (`local._ConnectedToName`) (`/Game/TileSystem/Blueprints/ConnectionPoint.Name` _asconnection_point))
        (set `/Game/TileSystem/Blueprints/ConnectionPoint.ConnectedConnector` (`local._ConnectedFrom`) _asconnection_point)
        (set `/Game/TileSystem/Blueprints/ConnectionPoint.ConnectedConnector` _asconnection_point (`local._ConnectedFrom`)))))
  (`BlueprintGameplayTagLibrary.AddGameplayTag` (`self.OwnedTags`) (struct :`TagName` "TileAssigned"))
  (`self.InitDone`))

(fn `UserConstructionScript`)